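; Surveillance camera that detects tagged players in its cone, raises alarms and shocks the detected player.
; Cone overlaps set the detected player and toggle the MetaUI HUD of player controller index 5.
; State changes recolor a dynamic decal for Seeking, Analyzing or Alarm; Alarm shows a targeted shock beam and spawns a burst, Seeking hides the beam.
; The separate raise-alarm event calls the alarm dispatch and shows the HUD alarm.
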(event `self.OnStateChange`
  (params (newState :type "CameraState Enum" :default "kSeeking"))
  (switch `CameraState` newState
    (:`kSeeking`
      (`MaterialInstanceDynamic.SetVectorParameterValue` (`self.DecalMaterial`) "Color" (struct :`R` 0.065458 :`G` 0.953125 :`B` 0.025047 :`A` 1.0))
      (`self.EndShock`))
    (:`kAnalyzing`
      (`MaterialInstanceDynamic.SetVectorParameterValue` (`self.DecalMaterial`) "Color" (struct :`R` 0.880122 :`G` 0.953125 :`B` 0.122397 :`A` 1.0)))
    (:`kAlarm`
      (`MaterialInstanceDynamic.SetVectorParameterValue` (`self.DecalMaterial`) "Color" (struct :`R` 0.994792 :`G` 0.044776 :`A` 1.0))
      (`self.ShockPlayer`))))

(event `self.ReceiveBeginPlay`
  (bind _returnvalue (`KismetMaterialLibrary.CreateDynamicMaterialInstance` "/Game/SurveillanceCamera/AreaMaterial.AreaMaterial"))
  (bind _output_get (set `self.DecalMaterial` _returnvalue))
  (`DecalComponent.SetDecalMaterial` (`self.Decal`) _output_get)
  (`MaterialInstanceDynamic.SetVectorParameterValue` (`self.DecalMaterial`) "Color" (struct :`R` 0.065458 :`G` 0.953125 :`B` 0.025047 :`A` 1.0))
  (`SceneComponent.SetVisibility` (`self.Shock`) false false))

(event `self.SurveillanceCone.OnComponentBeginOverlap`
  (params (OverlappedComponent :type "PrimitiveComponent Object Reference") (OtherActor :type "Actor Object Reference") (OtherComp :type "PrimitiveComponent Object Reference") (OtherBodyIndex :type Integer) (bFromSweep :type Boolean) (SweepResult :type "HitResult Structure (by ref)"))
  (if (`self.ActorHasTag` OtherActor "Player")
    (set `self.detectedPlayer` OtherActor)
    (bind _asmeta_ui (cast `/Game/HUD/MetaUI` (`PlayerController.GetHUD` (`GameplayStatics.GetPlayerController` 5))))
    (`/Game/HUD/MetaUI.ShowInCameraRange` _asmeta_ui)))

(event `self.SurveillanceCone.OnComponentEndOverlap`
  (params (OverlappedComponent :type "PrimitiveComponent Object Reference") (OtherActor :type "Actor Object Reference") (OtherComp :type "PrimitiveComponent Object Reference") (OtherBodyIndex :type Integer))
  (if (`self.ActorHasTag` OtherActor "Player")
    (set `self.detectedPlayer` null)
    (bind _asmeta_ui (cast `/Game/HUD/MetaUI` (`PlayerController.GetHUD` (`GameplayStatics.GetPlayerController` 5))))
    (`/Game/HUD/MetaUI.HideMetaUI` _asmeta_ui)))

(event `self.OnRaiseAlarm`
  (`KismetSystemLibrary.PrintString` "Alarm")
  (`self.AlarmDispatch`)
  (bind _asmeta_ui (cast `/Game/HUD/MetaUI` (`PlayerController.GetHUD` (`GameplayStatics.GetPlayerController` 5))))
  (`/Game/HUD/MetaUI.ShowAlarm` _asmeta_ui))

(fn `EndShock`
  (`SceneComponent.SetVisibility` (`self.Shock`) false false))

(fn `ShockPlayer`
  (`|ExecutionSequence`
    (:`then_0`
      (`FXSystemComponent.SetActorParameter` (`self.Shock`) "EndPoint" (`self.detectedPlayer`))
      (`SceneComponent.SetVisibility` (`self.Shock`) true false))
    (:`then_1`
      (bind _returnvalue (`|SpawnActorFromClass` "/Game/Electricity/ElectricShockBurstBP.ElectricShockBurstBP_C" (`self.GetTransform` (`self.detectedPlayer`)) "Undefined" "OverrideRootScale" null null))
      (`FXSystemComponent.SetActorParameter` (`/Game/Electricity/ElectricShockBurstBP.ElectricBurst` _returnvalue) "Center" (`self.detectedPlayer`)))))

(fn `UserConstructionScript`)